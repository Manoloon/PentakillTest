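; BP_Usable is an interactable item that can be inspected, picked up and rotated through Blueprint interface events.
; Inspecting reveals a Hint for about a second and plays a one-time proximity sound.
; Pickup runs once, playing a sound, hiding the hint, deactivating the decal and disabling Sphere collision, without destroying the actor.
; Rotation events compose incoming rotations onto the actor's current one, and BPIGetData returns its Data.
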(event Custom|Event_RotatePitch
  (params (Rotation :type Rotator))
  (Transformation|SetActorRotation (Math|Rotator|CombineRotators (Transformation|GetActorRotation) Rotation)))

(event Custom|Event_RotateYaw
  (params (Z%20%28Yaw%29 :type Float%20%28single-precision%29))
  (Transformation|SetActorRotation (Math|Rotator|CombineRotators (Transformation|GetActorRotation) (Math|Rotator|MakeRotator 0.0 0.0 Z%20%28Yaw%29))))

(event EventBeginPlay)

(event EventBPIRotateYaw
  (params (newYaw :type Float%20%28single-precision%29))
  (CallFunction|EventRotateYaw newYaw))

(event EventBPIRotate
  (params (NewRotator :type Rotator :default "0, 0, 0"))
  (CallFunction|EventRotatePitch NewRotator))

(event EventBPIInspect
  (Development|SetHiddeninGame (Variables|Default|Gethint) false false)
  (Utilities|FlowControl|Sequence
    (:then_0
      (Utilities|FlowControl|DoOnce false
        (:Completed
          (Audio|PlaySoundatLocation "/Game/Audio/SFX/NearPickup.NearPickup" (Transformation|GetActorLocation) "0, 0, 0" 1.0 1.0 0.0 0 0 0))))
    (:then_1
      (Utilities|FlowControl|Delay 1.0)
      (Development|SetHiddeninGame (Variables|Default|Gethint) true false))))

(event EventBPIPickItUp
  (bind _hint (Variables|Default|Gethint))
  (Utilities|FlowControl|DoOnce false
    (:Completed
      (Audio|PlaySoundatLocation "/Game/Audio/SFX/GetItem.GetItem" (Transformation|GetActorLocation) "0, 0, 0" 1.0 1.0 0.0 0 0 0)
      (Rendering|SetVisibility _hint false false)
      (Components|Activation|Deactivate _hint)
      (Components|Activation|Deactivate (Variables|Default|GetDecal))
      (Collision|SetCollisionEnabled (Variables|Default|GetSphere) "NoCollision"))))

(fn ConstructionScript)

(fn BPIGetData
  (return (Variables|Default|GetData)))