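; PentaGameMode is a game mode that runs the opening and ending transitions of a level.
; On BeginPlay it fades the camera and audio in while player input is disabled, then restores input in game-only mode with the cursor hidden.
; GameOver disables input, plays EndSequence with player and HUD hidden while fading out, then opens the m_endGame level after a delay.
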(event Custom|GameOver
  (Input|DisableInput (Game|Player|GetPlayerPawn 0) 0)
  (bind (_outactor _returnvalue) (Sequencer|Player|CreateLevelSequencePlayer (Variables|Default|GetEndSequence) (Utilities|Struct|MakeMovieSceneSequencePlaybackSettings false "(Value=0)" 1.0 0.0 false false false false true true false false)))
  (Sequencer|Player|Play (Variables|/Script/LevelSequence.LevelSequenceActor|GetSequencePlayer _outactor) :!class /Script/MovieScene.MovieSceneSequencePlayer)
  (CameraFades|StartCameraFade :self (Game|GetPlayerCameraManager 0) :ToAlpha 1.0 :Duration 2.0 :bShouldFadeAudio true :bHoldWhenFinished true)
  (Utilities|FlowControl|Delay 3.0)
  (Game|OpenLevel(byName) "m_endGame"))

(event EventBeginPlay
  (bind _returnvalue (Game|GetPlayerController 0))
  (Input|DisableInput (Game|Player|GetPlayerPawn 0) 0)
  (CameraFades|StartCameraFade :self (Game|GetPlayerCameraManager 0) :FromAlpha 1.0 :Duration 2.0 :bShouldFadeAudio true :bHoldWhenFinished true)
  (Utilities|FlowControl|Delay 3.0)
  (Input|EnableInput (Game|Player|GetPlayerPawn 0) 0)
  (Input|SetInputModeGameOnly _returnvalue)
  (Variables|/Script/Engine.PlayerController|SetbShowMouseCursor _returnvalue false))

(fn ConstructionScript)