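; BP_Door is a locked exit door that, when activated through interface events, unlocks, opens and loads the end-game level.
; Activation runs a timeline that spins the lock and fades in a point light, then plays a sound and swaps to an open-lock mesh.
; The open event changes the door material, disables player input and slides the mesh, while a delay precedes the level change.
; Inspecting briefly shows a hint.
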(event Custom|Event_OpenDoor
  (bind _staticmesh (Variables|Default|GetStaticMesh))
  (bind _returnvalue (Transformation|GetWorldLocation _staticmesh))
  (Rendering|Material|SetMaterial (Variables|Default|GetStaticMesh) 0 "/Game/PolygonPrototype/Materials/M_DoorOpen_Inst.M_DoorOpen_Inst")
  (Input|DisableInput (Game|GetPlayerController 0) 0)
  (bind _newtrack_0 (Timeline|Timeline_0 PlayFromStart)
    (:Update
      (Transformation|SetWorldLocation (Variables|Default|GetStaticMesh) (Math|Vector|Lerp(Vector) _returnvalue (+ _returnvalue "-100.000000,0.000000, 0") _newtrack_0) false false))
    (:Finished
      (Variables|Default|SetbIsOpen true))))

(event EventBeginPlay)

(event EventBPIActivate
  (bind _lock (Variables|Default|Getlock))
  (bind _newtrack_0 (Timeline|lock1 PlayFromStart)
    (:Update
      (Transformation|SetWorldRotation (Variables|Default|Getlock) (Math|Rotator|Lerp(Rotator) "0,90.000000, 0" "0,360.000000,0.000000" _newtrack_0) false false)
      (Rendering|Components|Light|SetIntensity (Variables|Default|GetPointLight) (Math|Float|Lerp 0.0 4e+02 _newtrack_0)))
    (:Finished
      (Audio|PlaySoundatLocation "/Game/Audio/SFX/OpenDoor.OpenDoor" (Transformation|GetActorLocation) "0, 0, 0" 1.0 1.0 0.0 0 0 0)
      (Components|StaticMesh|SetStaticMesh (Variables|Default|Getlock) "/Game/PolygonPrototype/Meshes/Icons/SM_Icon_Lock_Open_01.SM_Icon_Lock_Open_01")
      (CallFunction|EventOpenDoor)
      (Components|Activation|Deactivate (Variables|Default|GetHint))
      (Utilities|FlowControl|Delay 1.0)
      (Rendering|SetVisibility _lock false false)
      (Collision|SetCollisionEnabled _lock "NoCollision")
      (Game|OpenLevel(byName) "m_endGame"))))

(event EventBPIInspect
  (Development|SetHiddeninGame (Variables|Default|GetHint) false false)
  (Utilities|FlowControl|Delay 1.0)
  (Development|SetHiddeninGame (Variables|Default|GetHint) true false))

(fn ConstructionScript)