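; BP_Vela is a candle actor that other code can light or put out through an On interface event.
; The event toggles the glow ring mesh's visibility and switches the point light's intensity between a fixed value and zero.
; An IsIgnite flag guards both branches, so repeated calls with the same state change nothing.
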(event EventBeginPlay
  (|CallParentFunction))

(event Collision|EventActorBeginOverlap
  (params (OtherActor :type Actor%20Object%20Reference))
  (|CallParentFunction OtherActor) ; This node is disabled and will not be called.\nDrag off pins to build functionality.
)

(event EventTick
  (params (DeltaSeconds :type Float%20%28single-precision%29))
  (|CallParentFunction DeltaSeconds) ; This node is disabled and will not be called.\nDrag off pins to build functionality.
)

(event EventBPIon
  (params (On :type Boolean))
  (if On
    (if (not (Variables|Default|GetbIsIgnite?))
      (Variables|Default|SetbIsIgnite? true)
      (Rendering|SetVisibility (Variables|Default|GetSM_FX_Glow_Ring_01) true false)
      (Rendering|Components|Light|SetIntensity (Variables|Default|GetPointLight) 5e+02))
    (elif (Variables|Default|GetbIsIgnite?)
      (Variables|Default|SetbIsIgnite? false)
      (Rendering|SetVisibility (Variables|Default|GetSM_FX_Glow_Ring_01) false false)
      (Rendering|Components|Light|SetIntensity (Variables|Default|GetPointLight) 0.0))))

(fn ConstructionScript
  (|CallParentFunction))