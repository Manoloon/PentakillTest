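; Player controller that caches the controlled BP_Player on BeginPlay and handles the inventory and pause menu inputs.
; ShowInventory uses a FlipFlop to show and hide the inventory through the cached player.
; Pause uses a FlipFlop to open WG_Pause with Game and UI input and cursor, then remove it and restore game-only input.
; Closing the menu unpauses the game, but opening it does not set pause here.
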(event EventBeginPlay
  (bind _asbp_player (Utilities|Casting|CastToBP_Player (Pawn|GetControlledPawn)))
  (Variables|Default|SetAs%20BP%20Player _asbp_player))

(event EventTick
  (params (DeltaSeconds :type Float%20%28single-precision%29)))

(event Input|ActionEvents|InputActionShowInventory
  (params (Key :type Key%20Structure :default "None"))
  (:Pressed
    (bind _as_bp_player (Variables|Default|GetAs%20BP%20Player)
      (:then
        (Utilities|FlowControl|FlipFlop
          (:A
            (Default|ShowInventory _as_bp_player true))
          (:B
            (Default|ShowInventory _as_bp_player false))))
      (:else))))

(event Input|ActionEvents|InputActionPause
  (params (Key :type Key%20Structure :default "None"))
  (:Pressed
    (Utilities|FlowControl|FlipFlop
      (:A
        (bind _returnvalue (UserInterface|CreateWidget "/Game/UI/WG_Pause.WG_Pause_C" self))
        (bind _output_get (Variables|Default|SetPauseWidget _returnvalue))
        (UserInterface|Viewport|AddtoViewport _returnvalue 0)
        (Input|SetInputModeGameandUI self _output_get "LockOnCapture" false)
        (Variables|Default|SetbShowMouseCursor true))
      (:B
        (Utilities|IsValid (Variables|Default|GetPauseWidget)
          (:Is%20Valid
            (Widget|RemovefromParent (Variables|Default|GetPauseWidget))
            (Game|SetGamePaused false)
            (Input|SetInputModeGameOnly self)
            (Variables|Default|SetbShowMouseCursor false)))))))

(fn ConstructionScript)